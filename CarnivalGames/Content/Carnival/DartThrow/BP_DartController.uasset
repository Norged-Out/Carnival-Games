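; BP_DartController runs a carnival dart-throw minigame, starting a round when an XR pawn enters its start zone.
; StartGame resets the score, spawns a dart gun at the spawn point and binds to the gun's out-of-ammo and one found target's hit dispatchers.
; Functions update score and messages on a widget shown only while the player is in range.
; EndGame displays "Game Over" and expires the gun after a short delay.
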(event OnComponentBeginOverlap(StartZone)
  (params (OverlappedComponent :type Primitive%20Component%20Object%20Reference) (OtherActor :type Actor%20Object%20Reference) (OtherComp :type Primitive%20Component%20Object%20Reference) (OtherBodyIndex :type Integer) (bFromSweep :type Boolean) (SweepResult :type Hit%20Result%20Structure%20%28by%20ref%29))
  (Utilities|Casting|CastToBP_XRPawn OtherActor)
  (Variables|Default|SetbPlayerInRange true)
  (Development|PrintString "Starting Dart Throw Game")
  (Rendering|SetVisibility (Variables|Default|GetScoreWidget) true false)
  (if (not (Variables|Default|GetbGameActive))
    (CallFunction|StartGame)))

(event OnComponentEndOverlap(StartZone)
  (params (OverlappedComponent :type Primitive%20Component%20Object%20Reference) (OtherActor :type Actor%20Object%20Reference) (OtherComp :type Primitive%20Component%20Object%20Reference) (OtherBodyIndex :type Integer))
  (Utilities|Casting|CastToBP_XRPawn OtherActor)
  (Variables|Default|SetbPlayerInRange false)
  (Development|PrintString "Exiting Dart Throw Game")
  (Rendering|SetVisibility (Variables|Default|GetScoreWidget) false false))

(fn ConstructionScript)

(fn StartGame
  (Variables|Default|SetbGameActive true)
  (Variables|Default|SetTotalScore 0)
  (CallFunction|DisplayMessage "Dart Throw")
  (CallFunction|SpawnGun)
  (bind _returnvalue (Actor|GetActorOfClass "/Game/Carnival/DartThrow/BP_Target.BP_Target_C"))
  (EventDispatchers|BindEventtoOnTargetHit _returnvalue (EventDispatchers|CreateEvent :!event UpdateScore)))

(fn EndGame
  (Variables|Default|SetbGameActive false)
  (Actor|SetLifeSpan (Variables|Default|GetGun) 2.0)
  (CallFunction|DisplayMessage "Game Over"))

(fn SpawnGun
  (bind _gunspawnpoint (Variables|Default|GetGunSpawnPoint))
  (bind _returnvalue (Transformation|GetWorldTransform _gunspawnpoint))
  (bind (_location _rotation _scale) (Math|Transform|BreakTransform _returnvalue))
  (bind _returnvalue_2 (Game|SpawnActorfromClass "/Game/Carnival/DartThrow/BP_DartGun.BP_DartGun_C" (Math|Transform|MakeTransform _location "90.000000,180.000000,0.000000" _scale) "Undefined" "MultiplyWithRoot" 0 0))
  (bind _output_get (Variables|Default|SetGun _returnvalue_2))
  (EventDispatchers|BindEventtoOnOutOfAmmo _output_get (EventDispatchers|CreateEvent :!event EndGame)))

(fn UpdateScore
  (params (givenScore :type Integer))
  (Variables|Default|SetTotalScore (+ givenScore (Variables|Default|GetTotalScore)))
  (bind _aswbp_dart_score (Utilities|Casting|CastToWBP_GameScore (UserInterface|GetUserWidgetObject (Variables|Default|GetScoreWidget))))
  (Default|SetNewScore _aswbp_dart_score (Variables|Default|GetTotalScore)))

(fn DisplayMessage
  (params (inText :type Text))
  (bind _aswbp_dart_score (Utilities|Casting|CastToWBP_GameScore (UserInterface|GetUserWidgetObject (Variables|Default|GetScoreWidget))))
  (Default|SetMessage _aswbp_dart_score inText))