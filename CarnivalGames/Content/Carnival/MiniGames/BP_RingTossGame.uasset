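; BP_RingTossGame is a carnival ring toss minigame Blueprint that tracks throws, landed rings and score.
; RegisterLand increments RingsLanded, adds ten to Score and prints a debug message.
; CalculateScore calls its parent version, then returns ten points per landed ring, independently of Score.
; RegisterThrow is unfinished: its RingsThrown setter has no connected value, and the increment node sits outside the execution flow.
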(fn CalculateScore
  (|CallParentFunction)
  (return (* (Variables|Default|GetRingsLanded) 10)))

(fn RegisterThrow
  (params (RingsThrown :type Integer))
  (Variables|Default|SetRingsThrown (stale _result)))

(fn RegisterLand
  (Variables|Default|SetRingsLanded (+ (Variables|Default|GetRingsLanded) 1))
  (Variables|Default|SetScore (+ (Variables|Default|GetScore) 10))
  (Development|PrintString 0 "RegisterLand CALLED"))