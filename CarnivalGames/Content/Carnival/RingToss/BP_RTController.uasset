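; Runs a VR carnival Ring Toss game, started when the XR pawn enters a start zone that also toggles the score widget.
; Spawns one randomly colored BP_Ring at a time, binding its OnScored event.
; OnRingUsed expires the thrown ring and spawns the next, or ends the game on a delay when none remain.
; UpdateScore feeds the running total to the widget and points to the carnival player state.
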(event OnComponentBeginOverlap(StartZone)
  (params (OverlappedComponent :type Primitive%20Component%20Object%20Reference) (OtherActor :type Actor%20Object%20Reference) (OtherComp :type Primitive%20Component%20Object%20Reference) (OtherBodyIndex :type Integer) (bFromSweep :type Boolean) (SweepResult :type Hit%20Result%20Structure%20%28by%20ref%29))
  (Utilities|Casting|CastToBP_XRPawn OtherActor)
  (Variables|Default|SetbPlayerInRange true)
  (Development|PrintString "Starting Ring Toss Game")
  (Rendering|SetVisibility (Variables|Default|GetScoreWidget) true false)
  (if (not (Variables|Default|GetbGameActive))
    (CallFunction|StartGame)))

(event OnComponentEndOverlap(StartZone)
  (params (OverlappedComponent :type Primitive%20Component%20Object%20Reference) (OtherActor :type Actor%20Object%20Reference) (OtherComp :type Primitive%20Component%20Object%20Reference) (OtherBodyIndex :type Integer))
  (Utilities|Casting|CastToBP_XRPawn OtherActor)
  (Variables|Default|SetbPlayerInRange false)
  (Development|PrintString "Exiting Ring Toss Game")
  (Rendering|SetVisibility (Variables|Default|GetScoreWidget) false false))

(fn ConstructionScript)

(fn StartGame
  (Variables|Default|SetbGameActive true)
  (Variables|Default|SetRingsRemaining (Variables|Default|GetRingsToSpawn))
  (Variables|Default|SetTotalScore 0)
  (CallFunction|SpawnRing)
  (CallFunction|DisplayMessage "Ring Toss"))

(fn EndGame
  (Variables|Default|SetbGameActive false)
  (CallFunction|DisplayMessage "Game Over"))

(fn OnRingUsed
  (Variables|Default|SetbHasActiveRing false)
  (Actor|SetLifeSpan (Variables|Default|GetRing) 1e+01)
  (bind _output_get (Variables|Default|SetRingsRemaining (- (Variables|Default|GetRingsRemaining) 1)))
  (if (<= _output_get 0)
    (Utilities|Time|SetTimerbyFunctionName 0 "End Game" 5.0)
    (else
      (CallFunction|SpawnRing))))

(fn SpawnRing
  (if (and (> (Variables|Default|GetRingsRemaining) 0) (not (Variables|Default|GetbHasActiveRing)))
    (bind _returnvalue (Game|SpawnActorfromClass "/Game/Carnival/RingToss/BP_Ring.BP_Ring_C" (Transformation|GetWorldTransform (Variables|Default|GetSpawnPoint)) "AlwaysSpawn" "MultiplyWithRoot" 0 (Utilities|Select :Index (Math|Random|RandomIntegerinRange 0 2) :Option%200 "/Game/Carnival/Assets/Rings/RingOrange.RingOrange" :Option%201 "/Game/Carnival/Assets/Rings/RingGreen.RingGreen" :Option%202 "/Game/Carnival/Assets/Rings/RingPurple.RingPurple") 0))
    (bind _output_get (Variables|Default|SetRing _returnvalue))
    (EventDispatchers|BindEventtoOnScored _output_get (EventDispatchers|CreateEvent :!event UpdateScore))
    (Variables|Default|SetbHasActiveRing true)
    (Development|PrintString "Spawned Ring!")))

(fn UpdateScore
  (params (Given%20Score :type Integer))
  (CallFunction|UpdateScoreCard Given%20Score)
  (Variables|Default|SetTotalScore (+ Given%20Score (Variables|Default|GetTotalScore)))
  (bind _aswbp_game_score (Utilities|Casting|CastToWBP_GameScore (UserInterface|GetUserWidgetObject (Variables|Default|GetScoreWidget))))
  (Default|SetNewScore _aswbp_game_score (Variables|Default|GetTotalScore)))

(fn DisplayMessage
  (params (inText :type Text))
  (bind _aswbp_game_score (Utilities|Casting|CastToWBP_GameScore (UserInterface|GetUserWidgetObject (Variables|Default|GetScoreWidget))))
  (Default|SetMessage _aswbp_game_score inText))

(fn UpdateScoreCard
  (params (Amount :type Integer))
  (bind _asbp_carnival_player_state (Utilities|Casting|CastToBP_CarnivalPlayerState (Variables|/Script/Engine.Controller|GetPlayerState (Game|GetPlayerController 0))))
  (Default|AddRingTossScore _asbp_carnival_player_state Amount)
  (bind _aswbp_scorecard (Utilities|Casting|CastToWBP_Scorecard (UserInterface|GetUserWidgetObject (Variables|Default|GetScoreWidget))))
  (Default|UpdateScoreGameWise _aswbp_scorecard "NewEnumerator0"))