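; A grabbable ring for the carnival ring toss game that scores after staying inside a score zone for two seconds.
; EnterScoreZone stores the zone's score and enables Tick, which accumulates hold time and then marks the ring as scored, printing the result.
; ExitScoreZone clears the timer and score and prints a miss.
; Tick is switched off on scoring or exit and back on when grabbed or entering a zone.
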(event OnGrabbed(GrabComponent)
  (Actor|Tick|SetActorTickEnabled true))

(event EventTick
  (params (DeltaSeconds :type Float%20%28single-precision%29))
  (CallFunction|UpdateHoldTime DeltaSeconds)
  (CallFunction|TryScoring))

(fn ConstructionScript)

(fn TryScoring
  (if (>= (Variables|Default|GetholdTime) 2.0)
    (Variables|Default|SetbHasScored true)
    (Development|PrintString "Score!")
    (Development|PrintString (Utilities|String|ToString(Integer) (Variables|Default|GetScore)))
    (Actor|Tick|SetActorTickEnabled false)))

(fn EnterScoreZone
  (params (currScore :type Integer))
  (Variables|Default|SetbInsideZone true)
  (Variables|Default|SetScore currScore)
  (Actor|Tick|SetActorTickEnabled true))

(fn ExitScoreZone
  (Variables|Default|SetbInsideZone false)
  (Variables|Default|SetholdTime 0.0)
  (Variables|Default|SetScore 0)
  (Development|PrintString "Missed!")
  (Actor|Tick|SetActorTickEnabled false))

(fn UpdateHoldTime
  (params (DeltaSeconds :type Float%20%28double-precision%29))
  (if (and (Variables|Default|GetbInsideZone) (not (Variables|Default|GetbHasScored)))
    (Variables|Default|SetholdTime (+ DeltaSeconds (Variables|Default|GetholdTime)))))