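; Player state for the carnival game that holds the player's Ring Toss and Dart Throw scores.
; Each Add function overwrites its score rather than accumulating it, prints a debug message, then calls NotifyScoreChanged with a game-type enum.
; GetTotalScore returns the sum of both scores.
; NotifyScoreChanged and SaveScore are empty stubs, with SaveScore's ring-toss assignment left unconnected.
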(event EventBeginPlay)

(event EventTick
  (params (DeltaSeconds :type Float%20%28single-precision%29)))

(fn ConstructionScript)

(fn SaveScore
  (params (GameType :type Name) (Score :type Integer)))

(fn AddRingTossScore
  (params (Amount :type Integer))
  (Variables|Default|SetRingTossScore Amount)
  (Development|PrintString "Adding ring score success")
  (CallFunction|NotifyScoreChanged "NewEnumerator0"))

(fn GetTotalScore
  (return (+ (Variables|Default|GetRingTossScore) (Variables|Default|GetDartThrowScore))))

(fn AddDartThrowScore
  (params (Amount :type Integer))
  (Variables|Default|SetDartThrowScore Amount)
  (Development|PrintString "Adding dart throw score success")
  (CallFunction|NotifyScoreChanged "NewEnumerator1"))

(fn NotifyScoreChanged
  (params (GameType :type E_CarnivalGame%20Enum :default "NewEnumerator0")))