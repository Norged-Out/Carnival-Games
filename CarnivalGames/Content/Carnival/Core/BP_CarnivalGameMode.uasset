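; Game mode for the carnival game that opens a scorecard screen and provides scoring math.
; On BeginPlay it creates WBP_Scorecard, adds it to the viewport, switches input to UI only and shows the mouse cursor.
; NormalizeScore converts a game score to a percentage of its maximum, and CalculateFinalScore blends Whack, Spin and Shoot scores as a weighted sum favoring Whack and Spin.
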(event EventBeginPlay
  (bind _returnvalue (UserInterface|CreateWidget "/Game/Carnival/UI/WBP_Scorecard.WBP_Scorecard_C" (Game|GetPlayerController 0)))
  (UserInterface|Viewport|AddtoViewport _returnvalue 0)
  (Input|SetInputModeUIOnly 0 _returnvalue "DoNotLock" false)
  (Variables|/Script/Engine.PlayerController|SetbShowMouseCursor (Game|GetPlayerController 0) true))

(fn ConstructionScript)

(fn NormalizeScore
  (params (GameScore :type Float%20%28double-precision%29) (MaxScore :type Float%20%28double-precision%29))
  (return (* (/ GameScore MaxScore) 1e+02)))

(fn CalculateFinalScore
  (params (Whack :type Float%20%28double-precision%29) (Spin :type Float%20%28double-precision%29) (Shoot :type Float%20%28double-precision%29))
  (return (+ (+ (* Whack 0.4) (* Spin 0.4)) (* Shoot 0.2))))