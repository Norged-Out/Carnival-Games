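; Carnival game instance that holds the player's token count and a ring toss game object.
; On Init it constructs a BP_RingTossGame and stores it in RingTossGame, with debug prints around the assignment.
; InitializeTokens sets the starting balance.
; DeductTokens is effectively empty: its check-and-subtract logic is disconnected and never runs.
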(event EventInit
  (bind _returnvalue (Game|ConstructObjectfromClass "/Game/Carnival/MiniGames/BP_RingTossGame.BP_RingTossGame_C"))
  (Development|PrintString "setting ring toss game")
  (Variables|Default|SetRingTossGame _returnvalue)
  (Development|PrintString "set succesful"))

(fn InitializeTokens
  (params (InitialTokens :type Integer))
  (Variables|Default|SetTokens InitialTokens))

(fn DeductTokens
  (params (Cost :type Integer)))