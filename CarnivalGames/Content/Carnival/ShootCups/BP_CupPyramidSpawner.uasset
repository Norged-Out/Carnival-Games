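; Spawner actor for the carnival Shoot Cups game that places the cups, named as a pyramid.
; On BeginPlay it spawns the cup class at each transform in CupTransforms, ignoring collisions, and stores the spawned actors in an array.
; ResetCups destroys any still-valid cups, clears the array and spawns a fresh set from the same transforms.
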(event EventBeginPlay
  (Development|PrintString "Spawner BeginPlay")
  (CallFunction|SpawnCups))

(fn ConstructionScript)

(fn SpawnCups
  (for _array_element (Variables|Default|GetCupTransforms)
    (bind _returnvalue (Game|SpawnActorfromClass (Variables|Default|GetCupClass) _array_element "AlwaysSpawn" "MultiplyWithRoot" 0 0))
    (Utilities|Array|Add (Variables|Default|GetSpawnedCups) _returnvalue)))

(fn ResetCups
  (for _array_element (Variables|Default|GetSpawnedCups)
    (Utilities|IsValid _array_element
      (:Is%20Valid
        (Actor|DestroyActor _array_element))))
  (Utilities|Array|Clear (Variables|Default|GetSpawnedCups))
  (CallFunction|SpawnCups))