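; Controller for the Cup Drops carnival game, which spawns a pyramid of BP_Cup actors at CupSpawnPoint on BeginPlay.
; A StartZone overlap by BP_XRPawn shows the score widget and starts the game if inactive, while leaving only hides the widget.
; UpdateScore and DisplayMessage feed WBP_GameScore.
; EndGame shows "Game Over" and gives the controller a short lifespan, though nothing here calls it or UpdateScore.
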(event OnComponentBeginOverlap(StartZone)
  (params (OverlappedComponent :type Primitive%20Component%20Object%20Reference) (OtherActor :type Actor%20Object%20Reference) (OtherComp :type Primitive%20Component%20Object%20Reference) (OtherBodyIndex :type Integer) (bFromSweep :type Boolean) (SweepResult :type Hit%20Result%20Structure%20%28by%20ref%29))
  (Utilities|Casting|CastToBP_XRPawn OtherActor)
  (Variables|Default|SetbPlayerInRange true)
  (Development|PrintString "Starting Cup Drops Game")
  (Rendering|SetVisibility (Variables|Default|GetScoreWidget) true false)
  (if (not (Variables|Default|GetbGameActive))
    (CallFunction|StartGame)))

(event OnComponentEndOverlap(StartZone)
  (params (OverlappedComponent :type Primitive%20Component%20Object%20Reference) (OtherActor :type Actor%20Object%20Reference) (OtherComp :type Primitive%20Component%20Object%20Reference) (OtherBodyIndex :type Integer))
  (Utilities|Casting|CastToBP_XRPawn OtherActor)
  (Variables|Default|SetbPlayerInRange false)
  (Development|PrintString "Exiting Cup Drops Game")
  (Rendering|SetVisibility (Variables|Default|GetScoreWidget) false false))

(event EventBeginPlay
  (CallFunction|SpawnCups))

(fn ConstructionScript)

(fn StartGame
  (Variables|Default|SetbGameActive true)
  (Variables|Default|SetTotalScore 0)
  (CallFunction|DisplayMessage "Cup Drops"))

(fn EndGame
  (Variables|Default|SetbGameActive false)
  (Actor|SetLifeSpan 2.0)
  (CallFunction|DisplayMessage "Game Over"))

(fn UpdateScore
  (params (givenScore :type Integer))
  (Variables|Default|SetTotalScore (+ givenScore (Variables|Default|GetTotalScore)))
  (bind _aswbp_game_score (Utilities|Casting|CastToWBP_GameScore (UserInterface|GetUserWidgetObject (Variables|Default|GetScoreWidget))))
  (Default|SetNewScore _aswbp_game_score (Variables|Default|GetTotalScore)))

(fn DisplayMessage
  (params (inText :type Text))
  (bind _aswbp_game_score (Utilities|Casting|CastToWBP_GameScore (UserInterface|GetUserWidgetObject (Variables|Default|GetScoreWidget))))
  (Default|SetMessage _aswbp_game_score inText))

(fn SpawnCups
  (bind _rowcount (Variables|Default|GetRowCount))
  (bind _cupspawnpoint (Variables|Default|GetCupSpawnPoint))
  (bind _returnvalue (Transformation|GetWorldTransform _cupspawnpoint))
  (bind _returnvalue_2 (- _rowcount 1))
  (bind (_location _rotation _scale) (Math|Transform|BreakTransform _returnvalue))
  (for _index (range 0 _returnvalue_2)
    (for _index_2 (range 0 (- _returnvalue_2 _index))
      (Game|SpawnActorfromClass "/Game/Carnival/ShootCups/BP_Cup.BP_Cup_C" (Math|Transform|MakeTransform (Math|Vector|MakeVector (+ (|XOffset _index _index_2) (.x _location)) (.y _location) (+ (|ZOffset _index) (.z _location))) _rotation _scale) "Undefined" "MultiplyWithRoot" 0 0))))