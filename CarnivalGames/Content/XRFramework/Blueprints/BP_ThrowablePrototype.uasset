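; Prototype VR throwable object that smooths release velocity so it can be thrown when dropped from the hand.
; While GrabComponent reports it held, Tick records MyObject's linear and angular physics velocities into small rolling buffers.
; On drop, the averages of those buffers replace the object's velocities.
; Unconnected logic for hand hiding and per-hand weapon input mapping contexts is present but never runs.
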(event OnGrabbed(GrabComponent)
  (Variables|Default|SetisHeld true))

(event OnDropped(GrabComponent)
  (bind _myobject (Variables|Default|GetmyObject))
  (Physics|SetPhysicsLinearVelocity _myobject (Math|Vector|GetVectorArrayAverage (Variables|Default|GetVelocityLog)) false "None")
  (Class|PrimitiveComponent|SetPhysicsAngularVelocityinRadians _myobject (Math|Vector|GetVectorArrayAverage (Variables|Default|GetAngularVLog)) false "None")
  (Variables|Default|SetisHeld false))

(event EventTick
  (params (DeltaSeconds :type Float%20%28single-precision%29))
  (bind _myobject (Variables|Default|GetmyObject))
  (if (Variables|Default|GetisHeld)
    (bind _returnvalue (Physics|GetPhysicsLinearVelocity _myobject "None"))
    (Utilities|Array|SetArrayElem (Variables|Default|GetVelocityLog) (Variables|Default|GetFlow%20Control) _returnvalue)
    (Utilities|Array|SetArrayElem (Variables|Default|GetAngularVLog) (Variables|Default|GetFlow%20Control) (Class|PrimitiveComponent|GetPhysicsAngularVelocityinRadians _myobject "None"))
    (if (> (Variables|Default|GetFlow%20Control) 4)
      (Variables|Default|SetFlow%20Control 0)
      (else
        (Math|Integer|IncrementInt (Variables|Default|GetFlow%20Control))))))

(fn ConstructionScript)